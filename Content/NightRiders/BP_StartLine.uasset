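; BP_StartLine is the Night Riders start line actor, which starts the race timing and acts as the finish trigger.
; BeginPlay caches the player controller and game mode, then calls StartRace on the controller through a near-instant timer.
; Any Box overlap by an actor not tagged "ai" ends the race, shows the win screen with race time, switches to UI input and stops engine sound.
; Lap-counting nodes are left disconnected.
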(event OnComponentBeginOverlap(Box)
  (params (OverlappedComponent :type Primitive%20Component%20Object%20Reference) (OtherActor :type Actor%20Object%20Reference) (OtherComp :type Primitive%20Component%20Object%20Reference) (OtherBodyIndex :type Integer) (bFromSweep :type Boolean) (SweepResult :type Hit%20Result%20Structure%20%28by%20ref%29))
  (bind _returnvalue (Game|GetPlayerController 0))
  (if (not (Actor|ActorHasTag OtherActor "ai"))
    (Default|EndRace (Variables|Default|GetPlayerController))
    (bind _returnvalue_2 (UserInterface|CreateWidget "/Game/NightRiders/UI/WBP_WinScreen.WBP_WinScreen_C"))
    (bind _output_get (Variables|Default|SetWinScreen _returnvalue_2))
    (UserInterface|Viewport|AddtoViewport _output_get 0)
    (Input|SetInputModeUIOnly _returnvalue 0 "DoNotLock" false)
    (Input|EnableInput _returnvalue)
    (Variables|/Script/Engine.PlayerController|SetbShowMouseCursor _returnvalue true)
    (Rendering|Components|TextRender|SetText (Variables|/Game/NightRiders/UI/WBP_WinScreen.WBP_WinScreen_C|GetTextBlock_raceTime (Variables|Default|GetWinScreen)) (Variables|/Game/NightRiders/Vehicles/PlayerController/BP_PlayerController.BP_PlayerController_C|GetRaceTimeAsText (Variables|Default|GetPlayerController)))
    (Audio|Components|Audio|Stop (Variables|/Game/NightRiders/Vehicles/Car_Porsche911_GT2RS/BP_MainCar.BP_MainCar_C|GetEngineSound (Variables|/Game/NightRiders/Vehicles/PlayerController/BP_PlayerController.BP_PlayerController_C|GetCar (Variables|Default|GetPlayerController))))))

(event Custom|StartRaceTimer
  (Utilities|FlowControl|DoOnce false
    (:Completed
      (Default|StartRace (Variables|Default|GetPlayerController)))))

(event EventBeginPlay
  (bind _asbp_player_controller (Utilities|Casting|CastToBP_PlayerController (Game|GetPlayerController 0)))
  (Variables|Default|SetPlayerController _asbp_player_controller)
  (bind _asbp_car_gamemode (Utilities|Casting|CastToBP_CarGamemode (Game|GetGameMode)))
  (Variables|Default|SetCarGamemode _asbp_car_gamemode)
  (Utilities|Time|SetTimerbyEvent (delegate Custom|StartRaceTimer) 0.001 false false 5.0))

(event Collision|EventActorBeginOverlap
  (params (OtherActor :type Actor%20Object%20Reference)))

(event EventTick
  (params (DeltaSeconds :type Float%20%28single-precision%29)))

(fn ConstructionScript)