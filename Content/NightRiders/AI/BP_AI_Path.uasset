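; BP_AI_Path is a spline-based path actor that supplies target locations for AI.
; GetClosestLocationToSpline projects the AI's world location onto the spline, adds AdditionalDistance along it, and returns that world-space point.
; The SideOfRoad input has no effect on the result, because the nodes that offset the point left or right along the spline's right vector are left unconnected.
; The event graph and construction script are empty.
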(event EventBeginPlay)

(event Collision|EventActorBeginOverlap
  (params (OtherActor :type Actor%20Object%20Reference)))

(event EventTick
  (params (DeltaSeconds :type Float%20%28single-precision%29)))

(fn ConstructionScript)

(fn GetClosestLocationtoSpline
  (params (AILocation :type Vector :default "0, 0, 0") (AdditionalDistance :type Float%20%28double-precision%29) (SideOfRoad :type Integer))
  (bind _spline (Variables|Default|GetSpline))
  (return (Spline|GetLocationatDistanceAlongSpline _spline (+ (Class|SplineComponent|GetDistanceAlongSplineatLocation _spline AILocation "World") AdditionalDistance) "World")))