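; AI vehicle Blueprint that drives itself along the nearest BP_SplineRoad, chosen at BeginPlay.
; Each tick it steers toward a speed-scaled look-ahead point on the spline, computed only inside the DebugSteering branch.
; A second look-ahead from that point brakes for upcoming bends, except at or below MinSpeed.
; Steering yaw error also sets target speed, which drives full forward or reverse throttle.
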(event EventBeginPlay
  (|CallParentFunction)
  (bind _outactors (Actor|GetAllActorsOfClass "/Game/NightRiders/AI/OLD_AIVehicleSystem/BP_SplineRoad.BP_SplineRoad_C"))
  (bind _splineactor (CallFunction|FindNearestSpline _outactors))
  (Variables|Default|SetDefaultSpline _splineactor)
  (Variables|Default|SetSplineActor (Variables|Default|GetDefaultSpline))
  (Variables|SpeedControl|SetDefaultMaxSpeed (Variables|SpeedControl|GetMaxSpeed)))

(event Collision|EventActorBeginOverlap
  (params (OtherActor :type Actor%20Object%20Reference))
  (|CallParentFunction OtherActor) ; This node is disabled and will not be called.\nDrag off pins to build functionality.
)

(event EventTick
  (params (DeltaSeconds :type Float%20%28single-precision%29))
  (|CallParentFunction DeltaSeconds)
  (Utilities|IsValid (Variables|Default|GetSplineActor)
    (:Is%20Valid
      (Utilities|FlowControl|Sequence
        (:then_0
          (bind _returnvalue (CallFunction|CalculateSteeringInput (Variables|Default|GetSplineActor)))
          (Class|ChaosVehicleMovementComponent|SetSteeringInput (Variables|Default|GetVehicleMovementComponent) _returnvalue)
          (bind _returnvalue_2 (CallFunction|CalculateBrakeInput (Variables|Default|GetSplineActor) (Variables|Default|GetOffsetTangentLocation)))
          (Class|ChaosVehicleMovementComponent|SetBrakeInput (Variables|Default|GetVehicleMovementComponent) _returnvalue_2))
        (:then_1
          (Variables|SpeedControl|SetTargetSpeed (Math|Float|MapRangeClamped (Math|Float|Absolute(Float) (Variables|Default|GetYawDelta)) 3e+01 5.0 (Variables|SpeedControl|GetMinSpeed) (Variables|SpeedControl|GetMaxSpeed)))
          (if (< (Class|ChaosVehicleMovementComponent|GetForwardSpeedMPH (Variables|Default|GetVehicleMovementComponent)) (Variables|SpeedControl|GetTargetSpeed))
            (Class|ChaosVehicleMovementComponent|SetThrottleInput (Variables|Default|GetVehicleMovementComponent) 1.0)
            (else
              (Class|ChaosVehicleMovementComponent|SetThrottleInput (Variables|Default|GetVehicleMovementComponent) -1.0))))))))

(fn ConstructionScript
  (|CallParentFunction))

(fn FindNearestSpline
  (params (SplineActors :type Array%20of%20BP%20Spline%20Road%20Object%20References))
  (bind _returnvalue (Transformation|GetActorLocation))
  (LocalVariables|SetDistance 0.0)
  (for (_array_element _array_index) SplineActors
    (if (== _array_index 0)
      (LocalVariables|SetDistance (Math|Vector|Distance(Vector) (Spline|FindLocationClosesttoWorldLocation (Variables|/Game/NightRiders/AI/OLD_AIVehicleSystem/BP_SplineRoad.BP_SplineRoad_C|GetSpline _array_element) _returnvalue "World") _returnvalue) :!label _label)
      (LocalVariables|SetNearestSpline _array_element)
      (elif (< (Math|Vector|Distance(Vector) (Spline|FindLocationClosesttoWorldLocation (Variables|/Game/NightRiders/AI/OLD_AIVehicleSystem/BP_SplineRoad.BP_SplineRoad_C|GetSpline _array_element) _returnvalue "World") _returnvalue) (LocalVariables|GetDistance))
        (goto _label))))
  (return (LocalVariables|GetNearestSpline)))

(fn CalculateSteeringInput
  (params (Spline :type BP%20Spline%20Road%20Object%20Reference))
  (bind _returnvalue (Transformation|GetActorLocation))
  (bind _returnvalue_2 (Transformation|GetActorLocation))
  (bind _returnvalue_3 (Transformation|GetActorRotation))
  (bind _vehiclemovementcomponent (Variables|Default|GetVehicleMovementComponent))
  (bind _returnvalue_4 (Class|SplineComponent|FindTangentClosesttoWorldLocation (Variables|/Game/NightRiders/AI/OLD_AIVehicleSystem/BP_SplineRoad.BP_SplineRoad_C|GetSpline Spline) _returnvalue "World"))
  (bind _returnvalue_5 (Class|ChaosVehicleMovementComponent|GetForwardSpeedMPH _vehiclemovementcomponent))
  (bind _returnvalue_6 (Math|Vector|Normalize _returnvalue_4))
  (bind _returnvalue_7 (* _returnvalue_5 1e+01))
  (bind _returnvalue_8 (+ 2.5e+02 _returnvalue_7))
  (bind _returnvalue_9 (* _returnvalue_6 _returnvalue_8))
  (bind _returnvalue_10 (+ _returnvalue_9 _returnvalue))
  (bind _returnvalue_11 (Spline|FindLocationClosesttoWorldLocation (Variables|/Game/NightRiders/AI/OLD_AIVehicleSystem/BP_SplineRoad.BP_SplineRoad_C|GetSpline Spline) _returnvalue_10 "World"))
  (bind _returnvalue_12 (Math|Rotator|FindLookatRotation _returnvalue_2 _returnvalue_11))
  (bind _returnvalue_13 (Math|Rotator|Delta(Rotator) _returnvalue_12 _returnvalue_3))
  (bind _output_get (Variables|Default|SetOffsetTangentLocation _returnvalue_11))
  (if (Variables|DebugControl|GetDebugSteering)
    (Rendering|Debug|DrawDebugSphere _output_get 25.0 12 "(R=1.000000,G=0.000000,B=0.009454,A=1.000000)" 0.0 1.0)
    (Rendering|Debug|DrawDebugArrow _returnvalue_2 _output_get 1.0 "(R=1.000000,G=0.027873,B=0.000000,A=1.000000)" 0.0 1e+01)
    (Variables|Default|SetYawDelta (.yaw _returnvalue_13))
    (return (Math|Float|MapRangeClamped (.yaw _returnvalue_13) -15.0 15.0 -1.0 1.0))))

(fn CalculateBrakeInput
  (params (Spline :type BP%20Spline%20Road%20Object%20Reference) (OriginLocation :type Vector))
  (bind _returnvalue (Transformation|GetActorLocation))
  (bind _vehiclemovementcomponent (Variables|Default|GetVehicleMovementComponent))
  (bind _returnvalue_2 (Class|SplineComponent|FindTangentClosesttoWorldLocation (Variables|/Game/NightRiders/AI/OLD_AIVehicleSystem/BP_SplineRoad.BP_SplineRoad_C|GetSpline Spline) OriginLocation "World"))
  (bind _returnvalue_3 (Class|ChaosVehicleMovementComponent|GetForwardSpeedMPH _vehiclemovementcomponent))
  (bind _returnvalue_4 (Math|Vector|Normalize _returnvalue_2))
  (bind _returnvalue_5 (Math|Float|Clamp(Float) _returnvalue_3 1.0 _returnvalue_3))
  (bind _returnvalue_6 (* _returnvalue_5 5e+01))
  (bind _returnvalue_7 (* _returnvalue_4 _returnvalue_6))
  (bind _returnvalue_8 (+ _returnvalue_7 OriginLocation))
  (bind _returnvalue_9 (Spline|FindLocationClosesttoWorldLocation (Variables|/Game/NightRiders/AI/OLD_AIVehicleSystem/BP_SplineRoad.BP_SplineRoad_C|GetSpline Spline) _returnvalue_8 "World"))
  (if (Variables|DebugControl|GetDebugBrake)
    (Rendering|Debug|DrawDebugSphere _returnvalue_9 25.0 12 "(R=0.000000,G=1.000000,B=0.171331,A=1.000000)" 0.0 1.0)
    (Rendering|Debug|DrawDebugArrow _returnvalue _returnvalue_9 1.0 "(R=0.000000,G=1.000000,B=0.208508,A=1.000000)" 0.0 1e+01))
  (LocalVariables|SetBrakingInput (Math|Float|MapRangeClamped (+ (Math|Float|Absolute(Float) (.yaw (Math|Rotator|Delta(Rotator) (Math|Rotator|FindLookatRotation _returnvalue _returnvalue_9) (Transformation|GetActorRotation)))) (/ (Math|Float|Absolute(Float) (Variables|Default|GetYawDelta)) 4.0)) 15.0 35.0 0.0 1.0))
  (if (<= (Class|ChaosVehicleMovementComponent|GetForwardSpeedMPH (Variables|Default|GetVehicleMovementComponent)) (Variables|SpeedControl|GetMinSpeed))
    (LocalVariables|SetBrakingInput 0.0))
  (return (LocalVariables|GetBrakingInput)))