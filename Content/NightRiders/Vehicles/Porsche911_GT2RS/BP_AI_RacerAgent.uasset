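; AI racer agent Blueprint for the Porsche 911 GT2RS in NightRiders, mostly a thin child of its parent class.
; Its construction script runs the parent's, then copies the spline from RoadSpline into Spline when that reference is valid.
; BeginPlay and Tick only forward to the parent, and GetCurrentSpeed is a stub that always returns zero.
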(event EventBeginPlay
  (|CallParentFunction))

(event Collision|EventActorBeginOverlap
  (params (OtherActor :type Actor%20Object%20Reference))
  (|CallParentFunction OtherActor) ; This node is disabled and will not be called.\nDrag off pins to build functionality.
)

(event EventTick
  (params (DeltaSeconds :type Float%20%28single-precision%29))
  (|CallParentFunction DeltaSeconds))

(fn ConstructionScript
  (|CallParentFunction)
  (bind _roadspline (Variables|Default|GetRoadSpline)
    (:then
      (Variables|Default|SetSpline (Variables|/Game/NightRiders/AI/BP_AI_Path.BP_AI_Path_C|GetSpline _roadspline)))
    (:else)))

(fn GetCurrentSpeed
  (return 0.0))