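; Main menu game mode for NightRiders that creates the main menu widget and shows it on screen at BeginPlay.
; It stores the widget, enables input for player controller 0 and shows the mouse cursor.
; An AnyKey press collapses the widget's start screen, with the gamepad and non-gamepad branches doing the same thing.
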(event EventBeginPlay
  (bind _returnvalue (Game|GetPlayerController 0))
  (bind _returnvalue_2 (UserInterface|CreateWidget "/Game/NightRiders/UI/Menu/WBP_Main_Menu.WBP_Main_Menu_C"))
  (bind _output_get (Variables|Default|SetNewVar _returnvalue_2))
  (UserInterface|Viewport|AddtoViewport _returnvalue_2 0)
  (Input|EnableInput _returnvalue)
  (Variables|/Script/Engine.PlayerController|SetbShowMouseCursor _returnvalue true))

(event EventTick
  (params (DeltaSeconds :type Float%20%28single-precision%29)))

(event Input|KeyboardEvents|AnyKey
  (params (Key :type Key%20Structure :default "None"))
  (:Pressed
    (if (Class|KismetInputLibrary|KeyIsGamepadKey Key)
      (Widget|SetVisibility (Variables|/Game/NightRiders/UI/Menu/WBP_Main_Menu.WBP_Main_Menu_C|GetWBP_StartScreen (Variables|Default|GetNewVar)) "Collapsed")
      (else
        (Widget|SetVisibility (Variables|/Game/NightRiders/UI/Menu/WBP_Main_Menu.WBP_Main_Menu_C|GetWBP_StartScreen (Variables|Default|GetNewVar)) "Collapsed")))))

(fn ConstructionScript)