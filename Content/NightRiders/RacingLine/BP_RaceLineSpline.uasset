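; Racing line actor that lays a trail of arrow meshes along a spline, built entirely in the construction script with no runtime logic.
; Arrow spacing comes from the mesh's bounding-box X length plus an offset, which sets how many arrows span the spline.
; Each arrow is a Hierarchical Instanced Static Mesh instance, raised by a vertical offset and rotated toward the next sample point.
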(event EventBeginPlay)

(event Collision|EventActorBeginOverlap
  (params (OtherActor :type Actor%20Object%20Reference)))

(event EventTick
  (params (DeltaSeconds :type Float%20%28single-precision%29)))

(fn ConstructionScript
  (bind _arrowmesh (Variables|Default|GetArrowMesh))
  (bind _returnvalue (StaticMesh|GetBoundingBox _arrowmesh))
  (Variables|Default|SetArrowLength (+ (.X (Math|Vector|BreakVector (- (.max _returnvalue) (.min _returnvalue)))) (Variables|Default|GetArrowOffset)))
  (Components|StaticMesh|SetStaticMesh (Variables|Default|GetHierarchicalInstancedStaticMesh) (Variables|Default|GetArrowMesh))
  (for _index (range 0 (Math|Float|Floor (/ (Spline|GetSplineLength (Variables|Default|GetSpline)) (Variables|Default|GetArrowLength))))
    (Components|InstancedStaticMesh|AddInstance (Variables|Default|GetHierarchicalInstancedStaticMesh) (Math|Transform|MakeTransform (Math|Vector|MakeVector (.X (Math|Vector|BreakVector (Spline|GetLocationatDistanceAlongSpline (Variables|Default|GetSpline) (* _index (Variables|Default|GetArrowLength)) "Local"))) (.Y (Math|Vector|BreakVector (Spline|GetLocationatDistanceAlongSpline (Variables|Default|GetSpline) (* _index (Variables|Default|GetArrowLength)) "Local"))) (+ (.Z (Math|Vector|BreakVector (Spline|GetLocationatDistanceAlongSpline (Variables|Default|GetSpline) (* _index (Variables|Default|GetArrowLength)) "Local"))) (Variables|Default|GetArrowVerticalOffset))) (Math|Rotator|MakeRotfromX (- (Spline|GetLocationatDistanceAlongSpline (Variables|Default|GetSpline) (* (+ _index 1) (Variables|Default|GetArrowLength)) "Local") (Spline|GetLocationatDistanceAlongSpline (Variables|Default|GetSpline) (* _index (Variables|Default|GetArrowLength)) "Local"))) "1.000000,1.000000,1.000000") false)))