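; BP_RaceBarrierSpline is a spline actor that lays a row of arrow meshes for a race barrier, built entirely in the construction script.
; It spaces hierarchical instanced meshes by mesh length plus offset, lifts them vertically and aims each at the next spline sample.
; It adjusts ColouringArray toward the spline point count.
; GetColourWeight derives a weight from neighbouring point values, written to each instance's custom data.
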(event EventBeginPlay)

(event Collision|EventActorBeginOverlap
  (params (OtherActor :type Actor%20Object%20Reference)))

(event EventTick
  (params (DeltaSeconds :type Float%20%28single-precision%29)))

(fn ConstructionScript
  (bind _arrowmesh (Variables|Default|GetArrowMesh))
  (bind _colouringarray (Variables|Default|GetColouringArray))
  (bind _spline (Variables|Default|GetSpline))
  (bind _returnvalue (Utilities|Array|Length _colouringarray))
  (bind _returnvalue_2 (StaticMesh|GetBoundingBox _arrowmesh))
  (bind _returnvalue_3 (Spline|GetNumberOfSplinePoints _spline))
  (Utilities|FlowControl|Sequence
    (:then_0
      (Variables|Default|SetArrowLength (+ (.X (Math|Vector|BreakVector (- (.max _returnvalue_2) (.min _returnvalue_2)))) (Variables|Default|GetArrowOffset)))
      (Components|StaticMesh|SetStaticMesh (Variables|Default|GetHierarchicalInstancedStaticMesh) (Variables|Default|GetArrowMesh))
      (for _index (range 0 (Math|Float|Floor (/ (Spline|GetSplineLength (Variables|Default|GetSpline)) (Variables|Default|GetArrowLength))))
        (Components|InstancedStaticMesh|AddInstance (Variables|Default|GetHierarchicalInstancedStaticMesh) (Math|Transform|MakeTransform (Math|Vector|MakeVector (.X (Math|Vector|BreakVector (Spline|GetLocationatDistanceAlongSpline (Variables|Default|GetSpline) (* _index (Variables|Default|GetArrowLength)) "Local"))) (.Y (Math|Vector|BreakVector (Spline|GetLocationatDistanceAlongSpline (Variables|Default|GetSpline) (* _index (Variables|Default|GetArrowLength)) "Local"))) (+ (.Z (Math|Vector|BreakVector (Spline|GetLocationatDistanceAlongSpline (Variables|Default|GetSpline) (* _index (Variables|Default|GetArrowLength)) "Local"))) (Variables|Default|GetArrowVerticalOffset))) (Math|Rotator|MakeRotfromX (- (Spline|GetLocationatDistanceAlongSpline (Variables|Default|GetSpline) (* (+ _index 1) (Variables|Default|GetArrowLength)) "Local") (Spline|GetLocationatDistanceAlongSpline (Variables|Default|GetSpline) (* _index (Variables|Default|GetArrowLength)) "Local"))) "1.000000,1.000000,1.000000") false)))
    (:then_1
      (if (> _returnvalue_3 _returnvalue)
        (for _index_2 (range (- _returnvalue 1) (- _returnvalue_3 1))
          (Utilities|Array|Add (Variables|Default|GetColouringArray) 0.0))
        (else
          (for _index_3 (range _returnvalue_3 _returnvalue_3)
            (Utilities|Array|RemoveIndex (Variables|Default|GetColouringArray) _index_3)))))
    (:then_2
      (for _index_4 (range 0 (Math|Float|Floor (/ (Spline|GetSplineLength (Variables|Default|GetSpline)) (Variables|Default|GetArrowLength))))
        (Components|InstancedStaticMesh|SetCustomDataValue (Variables|Default|GetHierarchicalInstancedStaticMesh) _index_4 0 (CallFunction|GetColourWeight (Spline|GetLocationatDistanceAlongSpline (Variables|Default|GetSpline) (* _index_4 (Variables|Default|GetArrowLength)) "World")) false)))))

(fn GetColourWeight
  (params (Location :type Vector))
  (bind _spline (Variables|Default|GetSpline))
  (bind _returnvalue (Class|SplineComponent|FindInputKeyClosesttoWorldLocation _spline Location))
  (bind _returnvalue_2 (Math|Float|Floor _returnvalue))
  (LocalVariables|SetP1 _returnvalue_2)
  (LocalVariables|SetP2 (+ _returnvalue_2 1))
  (LocalVariables|SetWeight (Math|Float|%(Float) _returnvalue (- (Utilities|Array|Get(acopy) (Variables|Default|GetColouringArray) (LocalVariables|GetP2)) (Utilities|Array|Get(acopy) (Variables|Default|GetColouringArray) (LocalVariables|GetP1)))))
  (bind _output_get (LocalVariables|SetFinalW (+ (Utilities|Array|Get(acopy) (Variables|Default|GetColouringArray) (LocalVariables|GetP1)) (* (LocalVariables|GetWeight) (LocalVariables|GetDifferenceWeight)))))
  (return _output_get))